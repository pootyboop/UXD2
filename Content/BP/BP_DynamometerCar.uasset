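; BP_DynamometerCar is a dynamometer car that displays its speed and plays track noise while extending its parent's behavior.
; Each tick it pushes MPH, formatted to one decimal, into a W_MPH widget and applies the track volume multiplier to the noise.
; StartMoving fades in the noise and swaps the start screen for a stop tip; EndMoving restores the screens without stopping the audio itself.
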(event `self.ReceiveTick`
  (params (DeltaSeconds :type "Float (single-precision)"))
  (`parent.ReceiveTick` DeltaSeconds)
  (`self.updateMPHWidget`)
  (`AudioComponent.SetVolumeMultiplier` (`self.Track Noise`) (`self.trackVolumeMultiplier`)))

(event `self.StartMoving`
  (`AudioComponent.FadeIn` (`self.Track Noise`) 5.0 1.0 0.0 "Linear")
  (`SceneComponent.SetVisibility` (`self.StartScreen`) false false)
  (`SceneComponent.SetVisibility` (`self.StopTip`) true false))

(event `self.EndMoving`
  (`SceneComponent.SetVisibility` (`self.StartScreen`) true false)
  (`SceneComponent.SetVisibility` (`self.StopTip`) false false))

(fn `mphToText`
  (params (MPH :type "Float (double-precision)"))
  (returns (ReturnValue :type Text))
  (return (`KismetTextLibrary.Conv_DoubleToText` MPH "HalfToEven" false true 1 324 1 1)))

(fn `printMPH`
  (`KismetSystemLibrary.PrintString` (`KismetTextLibrary.Conv_TextToString` (`self.mphToText` (`self.MPH`))) true true (struct :`G` 0.66 :`B` 1.0 :`A` 1.0) 0.0))

(fn `updateMPHWidget`
  (`/Game/UI/W_MPH.setMPH` (cast `/Game/UI/W_MPH` (`WidgetComponent.GetUserWidgetObject` (`self.MPHWidget`)) :!pure true) (`self.mphToText` (`self.MPH`))))

(fn `UserConstructionScript`
  (`parent.UserConstructionScript`))