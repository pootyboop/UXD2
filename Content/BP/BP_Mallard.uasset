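; BP_Mallard is a child Blueprint for the Mallard, a moving object with steam, wind and whistle effects, apparently a locomotive.
; StartMoving activates the NWind and NSteam particles, sounds the whistle and starts a looping whistle timer.
; The timer's interval is randomized between min and max once per start, so it stays fixed until movement restarts.
; EndMoving deactivates the particles and clears the timer.
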(event `self.ReceiveBeginPlay`
  (`parent.ReceiveBeginPlay`))

(event `self.StartMoving`
  (`self.setParticlesActive` true)
  (`self.PlayWhistle`)
  (bind _returnvalue (`KismetSystemLibrary.K2_SetTimerDelegate` (delegate `PlayWhistle`) (`KismetMathLibrary.Lerp` (`self.minWhistleTime`) (`self.maxWhistleTime`) (`KismetMathLibrary.RandomFloat`)) true))
  (set `self.whistleTimer` _returnvalue))

(event `PlayWhistle`
  (`GameplayStatics.SpawnSoundAttached` "/Game/Assets/Audio/mallard-whistle.mallard-whistle" (`self.Whistle`) "None" (0.0 0.0 0.0) (struct) "KeepRelativeOffset" false 1.0 1.0 0.0 null null))

(event `self.EndMoving`
  (`self.setParticlesActive` false)
  (`KismetSystemLibrary.K2_ClearAndInvalidateTimerHandle` (`self.whistleTimer`)))

(fn `setParticlesActive`
  (params (bNewActive :type Boolean))
  (for _array_element (`|MakeArray` (`self.N_Wind`) (`self.N_Steam`))
    (`ActorComponent.SetActive` _array_element bNewActive false)))

(fn `UserConstructionScript`
  (`parent.UserConstructionScript`))