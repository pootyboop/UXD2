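; Train actor that starts on BeginPlay and rides along the spline of its assigned ActivePath until it reaches the end.
; A Start timeline scales Speed into CurrentSpeed, which Tick adds to Distance without delta time while setting location and rotation from the spline.
; A looping timer separately derives MPH from the distance moved between samples.
; Based on a linked YouTube tutorial.
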(event `self.ReceiveBeginPlay`
  ;[1 1 1] BASED ON: https://youtu.be/c6QwMAEsLRM
  (`self.StartTravel`)
  (`self.StartMPHTimer`))

(event `self.ReceiveTick`
  (params (DeltaSeconds :type "Float (single-precision)"))
  ;[1 1 1] BASED ON: https://youtu.be/c6QwMAEsLRM
  (`self.tryMove`))

(event `StartTravel`
  ;[1 1 1] BASED ON: https://youtu.be/c6QwMAEsLRM
  (`self.activePath`
    (:`then`
      (set `self.isMoving` true)
      (bind (_direction _start) (`Timeline|Start` :!via `PlayFromStart`)
        (:`Update`
          (set `self.currentSpeed` (* _start (`self.speed`))))))
    (:`else`
      (`KismetSystemLibrary.PrintString` "NO SPLINE PATH" true true (struct :`R` 1.0 :`G` 0.01 :`A` 1.0)))))

(event `StartMPHTimer`
  (set `self.lastPos` (`self.K2_GetActorLocation`))
  (`KismetSystemLibrary.K2_SetTimerDelegate` (delegate `UpdateMPHTimer`) (`self.MPHUpdateTime`) true))

(event `UpdateMPHTimer`
  (bind _milesperhour (`self.getMPH`))
  (set `self.MPH` _milesperhour))

(fn `getMPH`
  (returns (milesPerHour :type "Float (double-precision)"))
  (locals (currentPos :type "Vector Structure" :default (0.0 0.0 0.0)) (str :type String) (final :type "Float (double-precision)"))
  (bind _output_get (set `local.currentPos` (`self.K2_GetActorLocation`)))
  (set `local.final` (* (/ (/ (`KismetMathLibrary.Vector_Distance` _output_get (`self.lastPos`)) 160934.0) (`self.MPHUpdateTime`)) (/ 360.0 (`self.MPHUpdateTime`))))
  (set `self.lastPos` (`local.currentPos`))
  (return (`local.final`)))

(fn `moveAlong`
  (params (path :type "SplineComponent Object Reference") (dist :type "Float (double-precision)"))
  (bind (_returnvalue_roll _returnvalue_pitch _returnvalue_yaw) (`KismetMathLibrary.BreakRotator` (`SplineComponent.GetRotationAtDistanceAlongSpline` path dist "Local")))
  (`self.K2_SetActorLocationAndRotation` (`SplineComponent.GetLocationAtDistanceAlongSpline` path dist "World") (`KismetMathLibrary.MakeRotator` _returnvalue_roll _returnvalue_pitch _returnvalue_yaw)))

(fn `tryMove`
  (bind _distance (`self.distance`))
  (bind _spline (`/Game/Assets/BP/BP_TrainFollowSpline.Spline` (`self.activePath`)))
  (if (`self.isMoving`)
    (if (< _distance (`SplineComponent.GetSplineLength` _spline))
      (`self.moveAlong` _spline _distance)
      (set `self.distance` (+ (`self.distance`) (`self.currentSpeed`))))))

(fn `UserConstructionScript`)