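; BP_DynamometerCar is a car Blueprint that displays its speed on screen as a debug readout.
; Each Tick runs the parent's Tick, then prints the MPH value with zero duration so the text refreshes every frame.
; A helper formats the value to one decimal place with an MPH suffix; the speed itself is not calculated in these graphs, and MPHUpdateTime is unused.
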(event `self.ReceiveTick`
  (params (DeltaSeconds :type "Float (single-precision)"))
  (`parent.ReceiveTick` DeltaSeconds)
  (`self.printMPH`))

(fn `mphToString`
  (params (MPH :type "Float (double-precision)"))
  (returns (str :type String))
  (return (`KismetStringLibrary.Concat_StrStr` (`KismetTextLibrary.Conv_TextToString` (`KismetTextLibrary.Conv_DoubleToText` MPH "HalfToEven" false true 1 324 1 1)) " MPH")))

(fn `printMPH`
  (`KismetSystemLibrary.PrintString` (`self.mphToString` (`self.MPH`)) true true (struct :`G` 0.66 :`B` 1.0 :`A` 1.0) 0.0))

(fn `UserConstructionScript`
  (`parent.UserConstructionScript`))